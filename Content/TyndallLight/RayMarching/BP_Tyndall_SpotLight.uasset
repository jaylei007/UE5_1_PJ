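; Volumetric light shaft (Tyndall effect) actor that fakes a spot or directional light beam with a ray-marching material on a cube.
; The construction script sets the scene capture to perspective or orthographic to match the light type, targeting a new low-resolution R16f render target.
; That target feeds the matching dynamic material as its depth texture, alongside the light mask and shape, fade, density and step settings.
; All logic runs at construction.
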(event EventBeginPlay)

(event Collision|EventActorBeginOverlap
  (params (OtherActor :type Actor%20Object%20Reference)))

(event EventTick
  (params (DeltaSeconds :type Float%20%28single-precision%29)))

(fn ConstructionScript
  (bind _scenecapturecomponent2d (Variables|Default|GetSceneCaptureComponent2D))
  (if (Variables|Default|GetDirectionalLight)
    (Variables|/Script/Engine.SceneCaptureComponent2D|SetProjectionType _scenecapturecomponent2d "Orthographic")
    (Variables|/Script/Engine.SceneCaptureComponent2D|SetOrthoWidth _scenecapturecomponent2d (Variables|Default|GetWidth))
    (else
      (Variables|/Script/Engine.SceneCaptureComponent2D|SetProjectionType _scenecapturecomponent2d "Perspective")
      (Variables|/Script/Engine.SceneCaptureComponent2D|SetFOVAngle _scenecapturecomponent2d (Variables|Default|GetLightAngle))))
  (bind _returnvalue (Rendering|CreateRenderTarget2D 64 64 "RTF_R16f"))
  (Variables|/Script/Engine.SceneCaptureComponent2D|SetTextureTarget (Variables|Default|GetSceneCaptureComponent2D) _returnvalue)
  (bind _returnvalue_2 (Rendering|Material|CreateDynamicMaterialInstance (Variables|Default|GetCube) 0 (select (Variables|Default|GetDirectionalLight) "/Game/TyndallLight/RayMarching/Materials/M_SpotLight_Vol_Directional.M_SpotLight_Vol_Directional" "/Game/TyndallLight/RayMarching/Materials/M_SpotLight_Vol.M_SpotLight_Vol") "None" :!class /Script/Engine.PrimitiveComponent))
  (Rendering|Material|SetScalarParameterValue _returnvalue_2 "Angle" (/ (Variables|Default|GetLightAngle) 2.0) :!class /Script/Engine.MaterialInstanceDynamic)
  (Rendering|Material|SetScalarParameterValue _returnvalue_2 "Width" (/ (Variables|Default|GetWidth) 2.0) :!class /Script/Engine.MaterialInstanceDynamic)
  (Rendering|Material|SetScalarParameterValue _returnvalue_2 "LightLength" (Variables|Default|GetLightLength) :!class /Script/Engine.MaterialInstanceDynamic)
  (Rendering|Material|SetScalarParameterValue _returnvalue_2 "FadeDistance" (Variables|Default|GetFadeDistance) :!class /Script/Engine.MaterialInstanceDynamic)
  (Rendering|Material|SetScalarParameterValue _returnvalue_2 "Density" (Variables|Default|GetDensity) :!class /Script/Engine.MaterialInstanceDynamic)
  (Rendering|Material|SetScalarParameterValue _returnvalue_2 "MaxSteps" (Variables|Default|GetMaxSteps) :!class /Script/Engine.MaterialInstanceDynamic)
  (Rendering|Material|SetScalarParameterValue _returnvalue_2 "StepDistance" (Variables|Default|GetStepDistance) :!class /Script/Engine.MaterialInstanceDynamic)
  (Rendering|Material|SetTextureParameterValue _returnvalue_2 "Depth" (Variables|/Script/Engine.SceneCaptureComponent2D|GetTextureTarget (Variables|Default|GetSceneCaptureComponent2D)))
  (Rendering|Material|SetTextureParameterValue _returnvalue_2 "LightMask" (Variables|Default|GetLightMask)))