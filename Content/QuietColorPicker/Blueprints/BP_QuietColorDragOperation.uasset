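; Drag-and-drop operation for moving color buttons in the QuietColorPicker theme UI.
; On cancel, it casts the payload to a theme color button and returns it to the source theme at its stored panel index.
; Both cancel and drop hide the source theme's parent bin.
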(event EventDragCancelled
  (params (PointerEvent :type Pointer%20Event%20Structure%20%28by%20ref%29))
  (Utilities|IsValid (Variables|Default|GetSourceTheme)
    (:Is%20Valid
      (bind _aswbp_quiet_theme_color_button (Utilities|Casting|CastToWBP_QuietThemeColorButton (Variables|Default|GetPayload)))
      (Default|ReturnDraggedButton (Variables|Default|GetSourceTheme) _aswbp_quiet_theme_color_button (Variables|Default|GetSourcePanelIndex))
      (Default|ShowParentBin (Variables|Default|GetSourceTheme) false))))

(event EventDrop
  (params (PointerEvent :type Pointer%20Event%20Structure%20%28by%20ref%29))
  (Utilities|IsValid (Variables|Default|GetSourceTheme)
    (:Is%20Valid
      (Default|ShowParentBin (Variables|Default|GetSourceTheme) false))))