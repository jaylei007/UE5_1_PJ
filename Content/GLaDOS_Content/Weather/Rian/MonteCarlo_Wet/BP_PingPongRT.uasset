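; Ping-pong render target Blueprint that runs iterative random sampling, apparently for a Monte Carlo wetness effect.
; BeginPlay creates sampler and present material instances and clears the three render targets.
; Each Tick repeatedly feeds the sampler a random UV and alternates RT_A and RT_B as previous texture and draw target.
; The present material then draws to RT_Final; a note flags that Begin Draw should replace the current draw call.
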(event EventBeginPlay
  (bind _returnvalue (Rendering|Material|CreateDynamicMaterialInstance "/Game/GLaDOS_Content/Weather/Rian/MonteCarlo_Wet/M_Present.M_Present" "None" "None" :!class /Script/Engine.KismetMaterialLibrary))
  (Variables|Default|SetPresentMat _returnvalue)
  (bind _returnvalue_2 (Rendering|Material|CreateDynamicMaterialInstance "/Game/GLaDOS_Content/Weather/Rian/MonteCarlo_Wet/M_Sampler.M_Sampler" "None" "None" :!class /Script/Engine.KismetMaterialLibrary))
  (Variables|Default|SetSamplerMat _returnvalue_2)
  (Rendering|ClearRenderTarget2D "/Game/GLaDOS_Content/Weather/Rian/MonteCarlo_Wet/RT_A.RT_A")
  (Rendering|ClearRenderTarget2D "/Game/GLaDOS_Content/Weather/Rian/MonteCarlo_Wet/RT_B.RT_B")
  (Rendering|ClearRenderTarget2D "/Game/GLaDOS_Content/Weather/Rian/MonteCarlo_Wet/RT_Final.RT_Final"))

(event EventTick
  (params (DeltaSeconds :type Float%20%28single-precision%29))
  (bind _samplermat (Variables|Default|GetSamplerMat))
  (bind _samplermat_2 (Variables|Default|GetSamplerMat))
  (for _index (range 0 (Variables|Default|GetTimes))
    (Rendering|Material|SetVectorParameterValue (Variables|Default|GetSamplerMat) "uv" (Utilities|Struct|MakeLinearColor (Math|Random|RandomFloatinRange 0.0 1.0) (Math|Random|RandomFloatinRange 0.0 1.0) 0.0 1.0) :!class /Script/Engine.MaterialInstanceDynamic)
    (if (> (Math|Integer|%(Integer) _index 2) 0)
      (Rendering|Material|SetTextureParameterValue _samplermat_2 "LastTex" "/Game/GLaDOS_Content/Weather/Rian/MonteCarlo_Wet/RT_B.RT_B")
      (Rendering|DrawMaterialtoRenderTarget "/Game/GLaDOS_Content/Weather/Rian/MonteCarlo_Wet/RT_A.RT_A" _samplermat)
      (else
        (Rendering|Material|SetTextureParameterValue _samplermat_2 "LastTex" "/Game/GLaDOS_Content/Weather/Rian/MonteCarlo_Wet/RT_A.RT_A")
        (Rendering|DrawMaterialtoRenderTarget "/Game/GLaDOS_Content/Weather/Rian/MonteCarlo_Wet/RT_B.RT_B" _samplermat))))
  (Rendering|Material|SetScalarParameterValue (Variables|Default|GetPresentMat) "Times" (Math|Float|MakeLiteralFloat (Variables|Default|GetValue)) :!class /Script/Engine.MaterialInstanceDynamic)
  ;[1 0 0] Comment
  (Rendering|DrawMaterialtoRenderTarget "/Game/GLaDOS_Content/Weather/Rian/MonteCarlo_Wet/RT_Final.RT_Final" (Variables|Default|GetPresentMat)) ; 应该用begin draw函数代替
)

(fn ConstructionScript)