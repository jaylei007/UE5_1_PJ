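; Directional light actor for a custom render pipeline (CRP), publishing light direction and an orthographic light-space camera to materials.
; The construction script writes the negated Arrow forward vector and hand-built view and projection matrix rows into MPC_CRP_DirectinalLight.
; The view comes from the Arrow's axes and location; the projection scales X and flipped Y by the SceneCapture2D OrthoWidth, zeroing depth.
; The capture hides this actor, and nothing updates at runtime.
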(event EventBeginPlay)

(event Collision|EventActorBeginOverlap
  (params (OtherActor :type Actor%20Object%20Reference)))

(event EventTick
  (params (DeltaSeconds :type Float%20%28single-precision%29)))

(fn ConstructionScript
  (bind (_viewx _viewy _viewz _vieww) (CallFunction|BuildViewMatrix))
  (bind (_projx _projy _projz _projw) (CallFunction|BuildProjectionMatrix))
  (Variables|/Script/Engine.SceneCaptureComponent|SetHiddenActors (Variables|Default|GetSceneCaptureComponent2D) (Utilities|Array|MakeArray self))
  (Rendering|Material|SetVectorParameterValue "/Game/GLaDOS_Content/RenderingPipeline/LightAndShadow/DirectinalLight/MPC_CRP_DirectinalLight.MPC_CRP_DirectinalLight" "LightVector" (Math|Conversions|ToLinearColor(Vector) (* (Math|Vector|GetForwardVector (Variables|Default|GetArrow)) -1.0)) :!class /Script/Engine.KismetMaterialLibrary)
  (Utilities|FlowControl|Sequence
    (:then_0
      (Rendering|Material|SetVectorParameterValue "/Game/GLaDOS_Content/RenderingPipeline/LightAndShadow/DirectinalLight/MPC_CRP_DirectinalLight.MPC_CRP_DirectinalLight" "ViewX" (Math|Conversions|ToLinearColor(Vector) _viewx) :!class /Script/Engine.KismetMaterialLibrary)
      (Rendering|Material|SetVectorParameterValue "/Game/GLaDOS_Content/RenderingPipeline/LightAndShadow/DirectinalLight/MPC_CRP_DirectinalLight.MPC_CRP_DirectinalLight" "ViewY" (Math|Conversions|ToLinearColor(Vector) _viewy) :!class /Script/Engine.KismetMaterialLibrary)
      (Rendering|Material|SetVectorParameterValue "/Game/GLaDOS_Content/RenderingPipeline/LightAndShadow/DirectinalLight/MPC_CRP_DirectinalLight.MPC_CRP_DirectinalLight" "ViewZ" (Math|Conversions|ToLinearColor(Vector) _viewz) :!class /Script/Engine.KismetMaterialLibrary)
      (Rendering|Material|SetVectorParameterValue "/Game/GLaDOS_Content/RenderingPipeline/LightAndShadow/DirectinalLight/MPC_CRP_DirectinalLight.MPC_CRP_DirectinalLight" "ViewW" (Math|Conversions|ToLinearColor(Vector) _vieww) :!class /Script/Engine.KismetMaterialLibrary)
      (Rendering|Material|SetVectorParameterValue "/Game/GLaDOS_Content/RenderingPipeline/LightAndShadow/DirectinalLight/MPC_CRP_DirectinalLight.MPC_CRP_DirectinalLight" "ProjX" (Math|Conversions|ToLinearColor(Vector) _projx) :!class /Script/Engine.KismetMaterialLibrary)
      (Rendering|Material|SetVectorParameterValue "/Game/GLaDOS_Content/RenderingPipeline/LightAndShadow/DirectinalLight/MPC_CRP_DirectinalLight.MPC_CRP_DirectinalLight" "ProjY" (Math|Conversions|ToLinearColor(Vector) _projy) :!class /Script/Engine.KismetMaterialLibrary)
      (Rendering|Material|SetVectorParameterValue "/Game/GLaDOS_Content/RenderingPipeline/LightAndShadow/DirectinalLight/MPC_CRP_DirectinalLight.MPC_CRP_DirectinalLight" "ProjZ" (Math|Conversions|ToLinearColor(Vector) _projz) :!class /Script/Engine.KismetMaterialLibrary)
      (Rendering|Material|SetVectorParameterValue "/Game/GLaDOS_Content/RenderingPipeline/LightAndShadow/DirectinalLight/MPC_CRP_DirectinalLight.MPC_CRP_DirectinalLight" "ProjW" (Math|Conversions|ToLinearColor(Vector) _projw) :!class /Script/Engine.KismetMaterialLibrary))))

(fn BuildViewMatrix
  (bind _arrow (Variables|Default|GetArrow))
  (bind _returnvalue (Math|Vector|GetRightVector _arrow))
  (bind _returnvalue_2 (Math|Vector|GetUpVector _arrow))
  (bind _returnvalue_3 (Transformation|GetWorldLocation _arrow))
  (bind _returnvalue_4 (Math|Vector|GetForwardVector _arrow))
  (bind (_x _y _z) (Math|Vector|BreakVector _returnvalue_4))
  (bind (_x_2 _y_2 _z_2) (Math|Vector|BreakVector _returnvalue))
  (bind (_x_3 _y_3 _z_3) (Math|Vector|BreakVector _returnvalue_2))
  (return (Math|Vector|MakeVectorNetQuantize _x_2 _x_3 _x) (Math|Vector|MakeVectorNetQuantize _y_2 _y_3 _y) (Math|Vector|MakeVectorNetQuantize _z_2 _z_3 _z) (Math|Vector|MakeVectorNetQuantize (* (Math|Vector|DotProduct _returnvalue_3 _returnvalue) -1.0) (* (Math|Vector|DotProduct _returnvalue_3 _returnvalue_2) -1.0) (* (Math|Vector|DotProduct _returnvalue_3 _returnvalue_4) -1.0))))

(fn BuildProjectionMatrix
  (bind _scenecapturecomponent2d (Variables|Default|GetSceneCaptureComponent2D))
  (bind _orthowidth (Variables|/Script/Engine.SceneCaptureComponent2D|GetOrthoWidth _scenecapturecomponent2d))
  (return (Math|Vector|MakeVector (/ 2.0 _orthowidth) 0.0 0.0) (Math|Vector|MakeVector 0.0 (/ -2.0 _orthowidth) 0.0) (Math|Vector|MakeVector 0.0 0.0 0.0) (Math|Vector|MakeVector 0.0 0.0 0.0)))